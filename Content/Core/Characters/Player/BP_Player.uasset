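; BP_Player is the player character Blueprint, adding a camera spring arm effect for sprinting.
; BeginPlay caches the spring arm's target length as the default.
; Sprint start plays a timeline that lerps the arm from that default to the sprint length, and sprint end reverses it.
; The timeline update also assigns SprintSpeed to itself, so no speed change happens in this graph.
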(event EventOnSprintStart
  (bind _newtrack_0 (Timeline|SpringArmSprintTimeline Play)
    (:Update
      (Variables|/Script/Engine.SpringArmComponent|SetTargetArmLength (Variables|Default|GetSpringArmComponent) (Math|Float|Lerp (Variables|SprintSettings|GetDefaultArmLength) (Variables|SprintSettings|GetSprintArmLength) _newtrack_0))
      (Variables|Default|SetSprintSpeed (Variables|Default|GetSprintSpeed)))))

(event EventOnSprintEnd
  (bind _newtrack_0 (Timeline|SpringArmSprintTimeline Reverse)
    (:Update
      (Variables|/Script/Engine.SpringArmComponent|SetTargetArmLength (Variables|Default|GetSpringArmComponent) (Math|Float|Lerp (Variables|SprintSettings|GetDefaultArmLength) (Variables|SprintSettings|GetSprintArmLength) _newtrack_0))
      (Variables|Default|SetSprintSpeed (Variables|Default|GetSprintSpeed)))))

(event EventBeginPlay
  (Variables|SprintSettings|SetDefaultArmLength (Variables|/Script/Engine.SpringArmComponent|GetTargetArmLength (Variables|Default|GetSpringArmComponent)))
  (Variables|SprintSettings|SetDefaultArmLength (Variables|/Script/Engine.SpringArmComponent|GetTargetArmLength (Variables|Default|GetSpringArmComponent))))

(fn ConstructionScript)